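; Disco pirate character Blueprint that handles knockback, per-player sprite sets and bouncing for a flipbook-animated pirate.
; DamagedFallback tips the flipbook sideways and plays a timeline that lerps a swept move along Y, away from the attacker.
; SetFlipbooks passes a full animation set to SetFlipbooksImplementation by player index, with players 3 and 4 reusing the sets of 1 and 2.
; Bounce applies a large upward force through character movement.
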(event `self.DamagedFallback`
  (params (attackingPirate :type "Actor Object Reference"))
  (bind _flipbook (`self.flipbook`))
  (bind _damaged_origin_location (`self.Damaged Origin Location`))
  (set `self.Damaged Origin Location` (`self.K2_GetActorLocation`))
  (if (> (.y (`self.K2_GetActorLocation` attackingPirate)) (.y (`self.K2_GetActorLocation`)))
    (`SceneComponent.K2_SetRelativeRotation` _flipbook (struct :`Yaw` -90.0) false false)
    (set `self.Damaged Destination Location` (+ _damaged_origin_location (0.0 -200.0 0.0)))
    (bind (_direction _alpha) (`Timeline|Damaged Fallback` :!via `PlayFromStart` :!label _label)
      (:`Update`
        (`self.K2_SetActorLocation` (`KismetMathLibrary.MakeVector` (.x (`self.K2_GetActorLocation`)) (.y (`KismetMathLibrary.VLerp` (`self.Damaged Origin Location`) (`self.Damaged Destination Location`) _alpha)) (.z (`self.K2_GetActorLocation`))) true)))
    (else
      (`SceneComponent.K2_SetRelativeRotation` _flipbook (struct :`Yaw` 90.0) false false)
      (set `self.Damaged Destination Location` (+ _damaged_origin_location (0.0 200.0 0.0)))
      (goto _label :!via `PlayFromStart`))))

(event `self.SetFlipbooks`
  (params (playerIndex :type Integer))
  (bind _output_get (set `self.uniquePlayerIndex` playerIndex))
  (switch `int` _output_get
    (:`1`
      (`self.SetFlipbooksImplementation` "/Game/Flipbooks/Pirates/Pirate1/Pirate1Idle.Pirate1Idle" "/Game/Flipbooks/Pirates/Pirate1/Pirate1Walking.Pirate1Walking" "/Game/Flipbooks/Pirates/Pirate1/Pirate1Running.Pirate1Running" "/Game/Flipbooks/Pirates/Pirate1/Pirate1JumpingStart.Pirate1JumpingStart" "/Game/Flipbooks/Pirates/Pirate1/Pirate1JumpingLoop.Pirate1JumpingLoop" "/Game/Flipbooks/Pirates/Pirate1/Pirate1Attacking.Pirate1Attacking" "/Game/Flipbooks/Pirates/Pirate1/Pirate1Damaged.Pirate1Damaged" "/Game/Flipbooks/Pirates/Pirate1/Pirate1IdleDrinking.Pirate1IdleDrinking" "/Game/Flipbooks/Pirates/Pirate1/Pirate1RunningDrinking.Pirate1RunningDrinking" "/Game/Flipbooks/Pirates/Pirate1/Pirate1JumpingStartDrinking.Pirate1JumpingStartDrinking" "/Game/Flipbooks/Pirates/Pirate1/Pirate1JumpingLoopDrinking.Pirate1JumpingLoopDrinking" "/Game/Flipbooks/Pirates/Pirate1/Pirate1Stunned.Pirate1Stunned" "/Game/Flipbooks/Pirates/Pirate1/Pirate1Attacking.Pirate1Attacking" :!label _label_2))
    (:`2`
      (`self.SetFlipbooksImplementation` "/Game/Flipbooks/Pirates/Pirate2/Pirate2Idle.Pirate2Idle" "/Game/Flipbooks/Pirates/Pirate2/Pirate2Walking.Pirate2Walking" "/Game/Flipbooks/Pirates/Pirate2/Pirate2Running.Pirate2Running" "/Game/Flipbooks/Pirates/Pirate2/Pirate2JumpingStart.Pirate2JumpingStart" "/Game/Flipbooks/Pirates/Pirate2/Pirate2JumpingLoop.Pirate2JumpingLoop" "/Game/Flipbooks/Pirates/Pirate2/Pirate2Attacking.Pirate2Attacking" "/Game/Flipbooks/Pirates/Pirate2/Pirate2Damaged.Pirate2Damaged" "/Game/Flipbooks/Pirates/Pirate2/Pirate2IdleDrinking.Pirate2IdleDrinking" "/Game/Flipbooks/Pirates/Pirate2/Pirate2RunningDrinking.Pirate2RunningDrinking" "/Game/Flipbooks/Pirates/Pirate2/Pirate2JumpingStartDrinking.Pirate2JumpingStartDrinking" "/Game/Flipbooks/Pirates/Pirate2/Pirate2JumpingLoopDrinking.Pirate2JumpingLoopDrinking" "/Game/Flipbooks/Pirates/Pirate2/Pirate2Stunned.Pirate2Stunned" "/Game/Flipbooks/Pirates/Pirate2/Pirate2Attacking.Pirate2Attacking" :!label _label_3))
    (:`3`
      (goto _label_2))
    (:`4`
      (goto _label_3))))

(fn `Bounce!`
  (locals (OriginalJumpZ :type "Float (double-precision)" :default 0.0))
  (`CharacterMovementComponent.AddForce` (`self.CharacterMovement`) (0.0 0.0 50000000.0)))

(fn `UserConstructionScript`)