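; Camera actor blueprint that shows the mouse cursor and level HUD and relays player input to the disco pirate character.
; On BeginPlay it creates a GameLevelWidget and adds it to the player screen.
; Attack, Jump and Movement inputs call InitiateAttack, InitiateJump and MoveVertical on the pirate.
; Each input finds the pirate afresh by taking the first DiscoPirateBlueprint from GetAllActorsOfClass, with no caching or validity check.
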(event `self.ReceiveBeginPlay`
  (bind _returnvalue (`GameplayStatics.GetPlayerController` 0))
  (set `PlayerController.bShowMouseCursor` true _returnvalue)
  (bind _returnvalue_2 (`|CreateWidget` "/Game/Widgets/GameLevelWidget.GameLevelWidget_C" _returnvalue))
  (`UserWidget.AddToPlayerScreen` _returnvalue_2 0))

(event `InputAction|Attack`
  (params (Key :type "Key Structure" :default "AnyKey"))
  (:`Pressed`
    (bind _firstpirate (`self.GetFirstDiscoPirate`))
    (`DiscoPirate.InitiateAttack` _firstpirate)))

(event `InputAction|Jump`
  (params (Key :type "Key Structure" :default "AnyKey"))
  (:`Pressed`
    (bind _firstpirate (`self.GetFirstDiscoPirate`))
    (`DiscoPirate.InitiateJump` _firstpirate)))

(event `InputAxis|Movement`
  (params (AxisValue :type "Float (single-precision)"))
  (bind _firstpirate (`self.GetFirstDiscoPirate`))
  (`DiscoPirate.MoveVertical` _firstpirate AxisValue))

(fn `GetFirstDiscoPirate`
  (returns (FirstPIrate :type "/Game/Blueprints/DiscoPirateBlueprint Object Reference"))
  (bind _outactors (`GameplayStatics.GetAllActorsOfClass` "/Game/Blueprints/DiscoPirateBlueprint.DiscoPirateBlueprint_C"))
  (return (`KismetArrayLibrary.Array_Get` _outactors)))

(fn `UserConstructionScript`)