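; Cannonball projectile actor for a 2D Paper2D game, confined to the YZ plane and destroyed after its lifetime expires.
; On spawn it snaps X to zero and plays its initial flipbook once, then switches to a looping idle flipbook.
; Each tick it wraps around to the opposite side when it crosses the level's Y or Z boundaries.
; Its sphere overlap calls Attack on any DiscoPirate it touches, passing itself.
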(event `self.ReceiveBeginPlay`
  (`PaperFlipbookComponent.SetLooping` (`self.PaperFlipbook`) false)
  (`self.K2_SetActorLocation` (`KismetMathLibrary.MakeVector` 0.0 (.y (`self.K2_GetActorLocation`)) (.z (`self.K2_GetActorLocation`))))
  (`KismetSystemLibrary.Delay` (`self.LifeTime`))
  (`self.K2_DestroyActor`))

(event `self.ReceiveTick`
  (params (DeltaSeconds :type "Float (single-precision)"))
  (bind _level_z_boundary (`self.Level Z Boundary`))
  (bind _level_z_boundary_2 (`self.Level Z Boundary`))
  (bind _level_y_boundary (`self.Level Y Boundary`))
  (bind _level_y_boundary_2 (`self.Level Y Boundary`))
  (`|ExecutionSequence`
    (:`then_0`
      (if (> (.y (`self.K2_GetActorLocation`)) _level_y_boundary)
        (`self.K2_AddActorWorldOffset` (`KismetMathLibrary.MakeVector` 0.0 (* (* _level_y_boundary -1.0) 2.0)))
        (elif (< (.y (`self.K2_GetActorLocation`)) (* _level_y_boundary_2 -1.0))
          (`self.K2_AddActorWorldOffset` (`KismetMathLibrary.MakeVector` 0.0 (* _level_y_boundary_2 2.0))))))
    (:`then_1`
      (if (> (.z (`self.K2_GetActorLocation`)) _level_z_boundary)
        (`self.K2_AddActorWorldOffset` (`KismetMathLibrary.MakeVector` 0.0 0.0 (* (* _level_z_boundary -1.0) 2.0)))
        (elif (< (.z (`self.K2_GetActorLocation`)) (* _level_z_boundary_2 -1.0))
          (`self.K2_AddActorWorldOffset` (`KismetMathLibrary.MakeVector` 0.0 0.0 (* _level_z_boundary_2 2.0))))))))

(event `self.PaperFlipbook.OnFinishedPlaying`
  (bind _paperflipbook (`self.PaperFlipbook`))
  (`PaperFlipbookComponent.SetLooping` _paperflipbook true)
  (`PaperFlipbookComponent.SetFlipbook` _paperflipbook "/Game/Flipbooks/CannonBallIdle.CannonBallIdle"))

(event `self.Sphere.OnComponentBeginOverlap`
  (params (OverlappedComponent :type "PrimitiveComponent Object Reference") (OtherActor :type "Actor Object Reference") (OtherComp :type "PrimitiveComponent Object Reference") (OtherBodyIndex :type Integer) (bFromSweep :type Boolean) (SweepResult :type "HitResult Structure (by ref)"))
  (bind _asdisco_pirate (cast `DiscoPirate` OtherActor))
  (`DiscoPirate.Attack` _asdisco_pirate self))

(fn `UserConstructionScript`)