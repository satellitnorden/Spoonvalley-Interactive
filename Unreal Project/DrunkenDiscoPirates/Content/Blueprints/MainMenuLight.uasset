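; MainMenuLight is a Blueprint light, named for the main menu, that pulses in intensity and changes color at random.
; The LightPulsation timeline drives intensity from zero to a bright peak through its Alpha track.
; At BeginPlay and on each Loop event, it gets a random play rate and SetNewLightColor picks a color from LightColors.
; No graph call starts the timeline; only its play rate is set.
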(event `self.ReceiveBeginPlay`
  (`self.SetNewLightColor`)
  (`TimelineComponent.SetPlayRate` (`self.LightPulsation`) (`KismetMathLibrary.RandomFloatInRange` 0.5 5.0)))

(fn `SetNewLightColor`
  (bind _lightcolors (`self.LightColors`))
  (`LightComponent.SetLightColor` (`self.Light`) (`KismetArrayLibrary.Array_Get` _lightcolors (`KismetMathLibrary.RandomIntegerInRange` 0 (- (`KismetArrayLibrary.Array_Length` _lightcolors) 1))) true))

(fn `UserConstructionScript`)