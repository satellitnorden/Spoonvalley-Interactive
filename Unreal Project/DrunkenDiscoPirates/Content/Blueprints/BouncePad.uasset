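; Bounce pad actor that plays a flipbook animation and launches the DiscoPirate character that touches it.
; Overlapping the bounce box stops looping, swaps to the bounce flipbook and flags the pad as bouncing.
; When that flipbook finishes, it calls Bounce on the cast pirate, waits briefly, then restores the looping idle animation and clears the flag.
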(event `self.BounceBox.OnComponentBeginOverlap`
  (params (OverlappedComponent :type "PrimitiveComponent Object Reference") (OtherActor :type "Actor Object Reference") (OtherComp :type "PrimitiveComponent Object Reference") (OtherBodyIndex :type Integer) (bFromSweep :type Boolean) (SweepResult :type "HitResult Structure (by ref)"))
  (bind _bouncepadidle (`self.BouncePadIdle`))
  (bind _asdisco_pirate_blueprint (cast `/Game/Blueprints/DiscoPirateBlueprint` OtherActor))
  (`PaperFlipbookComponent.SetLooping` _bouncepadidle false)
  (`PaperFlipbookComponent.SetFlipbook` _bouncepadidle "/Game/Flipbooks/BouncePadFlipbook1.BouncePadFlipbook1")
  (set `self.IsBouncing` true))

(event `self.BouncePadIdle.OnFinishedPlaying`
  (bind _bouncepadidle (`self.BouncePadIdle`))
  (`/Game/Blueprints/DiscoPirateBlueprint.Bounce!` (stale `self.BounceBox.OnComponentBeginOverlap` _asdisco_pirate_blueprint))
  (`KismetSystemLibrary.Delay` 0.1)
  (`PaperFlipbookComponent.SetFlipbook` _bouncepadidle "/Game/Flipbooks/BouncePadFlipbook2.BouncePadFlipbook2")
  (`PaperFlipbookComponent.SetLooping` _bouncepadidle true)
  (`PaperFlipbookComponent.SetFlipbook` _bouncepadidle "/Game/Flipbooks/BouncePadIDle.BouncePadIdle")
  (`PaperFlipbookComponent.PlayFromStart` _bouncepadidle)
  (set `self.IsBouncing` false))

(fn `UserConstructionScript`)