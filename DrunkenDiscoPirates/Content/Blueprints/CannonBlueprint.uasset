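; Paper2D cannon that fires a cannonball when a DiscoPirate enters its trigger box while it is not already shooting.
; Overlap hides the ball flipbook and plays a one-shot fire animation, whose finish event spawns CannonballBlueprint at the Arrow transform with a sound.
; After a brief delay the cannon returns to its looping idle, then waits ReloadTime to show the ball again and clear IsShooting.
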(event `self.ReceiveBeginPlay`)

(event `self.ReceiveActorBeginOverlap`
  (params (OtherActor :type "Actor Object Reference")))

(event `self.ReceiveTick`
  (params (DeltaSeconds :type "Float (single-precision)")))

(event `self.Box.OnComponentBeginOverlap`
  (params (OverlappedComponent :type "PrimitiveComponent Object Reference") (OtherActor :type "Actor Object Reference") (OtherComp :type "PrimitiveComponent Object Reference") (OtherBodyIndex :type Integer) (bFromSweep :type Boolean) (SweepResult :type "HitResult Structure (by ref)"))
  (bind _paperflipbook (`self.PaperFlipbook`))
  (if (not (`self.IsShooting`))
    (cast `DiscoPirate` OtherActor)
    (`SceneComponent.SetHiddenInGame` (`self.PaperFlipbook1`) true false)
    (`PaperFlipbookComponent.SetLooping` _paperflipbook false)
    (`PaperFlipbookComponent.SetFlipbook` _paperflipbook "/Game/Flipbooks/CannonFireActive.CannonFireActive")
    (set `self.IsShooting` true)))

(event `self.PaperFlipbook.OnFinishedPlaying`
  (bind _paperflipbook1 (`self.PaperFlipbook1`))
  (bind _paperflipbook (`self.PaperFlipbook`))
  (`|SpawnActorFromClass` "/Game/Blueprints/CannonballBlueprint.CannonballBlueprint_C" (`SceneComponent.K2_GetComponentToWorld` (`self.Arrow`)) "Undefined" "OverrideRootScale")
  (`GameplayStatics.PlaySoundAtLocation` "/Game/Sounds/SoundCues/CannonFire.CannonFire")
  (`KismetSystemLibrary.Delay` 0.1)
  (`|ExecutionSequence`
    (:`then_0`
      (`PaperFlipbookComponent.SetFlipbook` _paperflipbook "/Game/Flipbooks/CannonFireActive2.CannonFireActive2"))
    (:`then_1`
      (`PaperFlipbookComponent.SetLooping` _paperflipbook true)
      (`PaperFlipbookComponent.SetFlipbook` _paperflipbook "/Game/Flipbooks/CannonFireIdle.CannonFireIdle")
      (`PaperFlipbookComponent.PlayFromStart` _paperflipbook))
    (:`then_2`
      (`KismetSystemLibrary.Delay` (`self.Reload Time`))
      (`GameplayStatics.PlaySoundAtLocation` "/Game/Sounds/SoundCues/CannonReload.CannonReload")
      (`PaperFlipbookComponent.SetLooping` _paperflipbook1 true)
      (`PaperFlipbookComponent.SetFlipbook` _paperflipbook1 "/Game/Flipbooks/CannonBallIdle.CannonBallIdle")
      (`SceneComponent.SetHiddenInGame` _paperflipbook1 false false)
      (`PaperFlipbookComponent.PlayFromStart` _paperflipbook1)
      (set `self.IsShooting` false))))

(fn `UserConstructionScript`)